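; Main player character with world-axis movement, sprint and speed-dependent jumps, viewed through fixed-angle cameras chosen by a Direction variable (left, front or other side).
; Tick moves a separate ActiveCamera actor toward that side's camera component with VInterpTo, using resettable DoOnce gates to set rotation once per switch and CameraChange to speed the transition.
; Movement axes remap per Direction, and held camera inputs offset spring-arm sockets to pan the view.
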(event Custom|ResetCameraLeftSide
  ;[1 1 1] Camera Controls
  ;;[1 1 1] Camera Change System
  (Utilities|FlowControl|DoOnce false) ; enters at Reset
)

(event Custom|ResetCameraRightSide
  ;[1 1 1] Camera Controls
  ;;[1 1 1] Camera Change System
  (Utilities|FlowControl|DoOnce false) ; enters at Reset
)

(event Custom|ResetCameraFrontSide
  ;[1 1 1] Camera Controls
  ;;[1 1 1] Camera Change System
  (Utilities|FlowControl|DoOnce false) ; enters at Reset
)

(event EventBeginPlay
  (bind _camera (Variables|Default|GetCamera))
  ;[1 1 1] Camera Controls
  ;;[1 1 1] First Action Camera Adjust
  (bind _outactors (Actor|GetAllActorsOfClass "/Game/Game_Files/Characters/Main_Character/ActiveCamera.ActiveCamera_C"))
  (Variables|Default|SetActiveCamera (Utilities|Array|Get(acopy) _outactors))
  (Game|Player|SetViewTargetwithBlend (Game|GetPlayerController 0) (Variables|Default|GetActiveCamera) 0.0 "VTBlend_Linear" 0.0 false)
  (Transformation|SetActorLocation (Variables|Default|GetActiveCamera) (Transformation|GetWorldLocation _camera) false false)
  (Transformation|SetActorRotation (Variables|Default|GetActiveCamera) (Transformation|GetWorldRotation _camera)))

(event EventTick
  (params (DeltaSeconds :type Float%20%28single-precision%29))
  ;[1 1 1] Camera Controls
  ;;[1 1 1] Camera Change System
  (Variables|Default|SetSpeedOfCharacter (Math|Vector|VectorLength (Variables|/Script/Engine.MovementComponent|GetVelocity (Variables|Character|GetCharacterMovement))))
  (if (Utilities|Enum|Equal(Enum) (Variables|Default|GetDirection) "LeftSide")
    (if (Variables|Default|GetCameraChange)
      (Variables|Default|SetSpeedOfVinterp 1e+03))
    (CallFunction|ResetCameraFrontSide)
    (CallFunction|ResetCameraRightSide)
    (Transformation|SetActorLocation (Variables|Default|GetActiveCamera) (Math|Interpolation|VInterpTo (Transformation|GetActorLocation (Variables|Default|GetActiveCamera)) (Transformation|GetWorldLocation (Variables|Default|GetCamera)) (Utilities|Time|GetWorldDeltaSeconds) (Variables|Default|GetSpeedOfVinterp)) false false)
    (Utilities|FlowControl|DoOnce false
      (:Completed
        (Transformation|SetActorRotation (Variables|Default|GetActiveCamera) (Transformation|GetWorldRotation (Variables|Default|GetCamera)))
        (Variables|Default|SetSpeedOfVinterp 1.5)
        (Variables|Default|SetCameraChange false)))
    (elif (Utilities|Enum|Equal(Enum) (Variables|Default|GetDirection) "FrontSide")
      (if (Variables|Default|GetCameraChange)
        (Variables|Default|SetSpeedOfVinterp 1e+03))
      (CallFunction|ResetCameraLeftSide)
      (CallFunction|ResetCameraRightSide)
      (Transformation|SetActorLocation (Variables|Default|GetActiveCamera) (Math|Interpolation|VInterpTo (Transformation|GetActorLocation (Variables|Default|GetActiveCamera)) (Transformation|GetWorldLocation (Variables|Default|GetCamera1)) (Utilities|Time|GetWorldDeltaSeconds) (Variables|Default|GetSpeedOfVinterp)) false false)
      (Utilities|FlowControl|DoOnce false
        (:Completed
          (Transformation|SetActorRotation (Variables|Default|GetActiveCamera) (Transformation|GetWorldRotation (Variables|Default|GetCamera1)))
          (Variables|Default|SetSpeedOfVinterp 1.5)
          (Variables|Default|SetCameraChange false)))
      (else
        (if (Variables|Default|GetCameraChange)
          (Variables|Default|SetSpeedOfVinterp 1e+03))
        (CallFunction|ResetCameraLeftSide)
        (CallFunction|ResetCameraFrontSide)
        (Transformation|SetActorLocation (Variables|Default|GetActiveCamera) (Math|Interpolation|VInterpTo (Transformation|GetActorLocation (Variables|Default|GetActiveCamera)) (Transformation|GetWorldLocation (Variables|Default|GetCamera2)) (Utilities|Time|GetWorldDeltaSeconds) (Variables|Default|GetSpeedOfVinterp)) false false)
        (Utilities|FlowControl|DoOnce false
          (:Completed
            (Transformation|SetActorRotation (Variables|Default|GetActiveCamera) (Transformation|GetWorldRotation (Variables|Default|GetCamera2)))
            (Variables|Default|SetSpeedOfVinterp 1.5)
            (Variables|Default|SetCameraChange false)))))))

(event Input|ActionEvents|InputActionSprint
  (params (Key :type Key%20Structure :default "None"))
  (bind _jumped (Variables|Default|GetJumped))
  (bind _charactermovement (Variables|Character|GetCharacterMovement))
  ;[1 1 1] Movemnet Controls
  (:Pressed
    (if (not _jumped)
      (Variables|/Script/Engine.CharacterMovementComponent|SetMaxWalkSpeed _charactermovement 3.5e+02)))
  (:Released
    (if (not _jumped)
      (Variables|/Script/Engine.CharacterMovementComponent|SetMaxWalkSpeed _charactermovement 225.0))))

(event Input|ActionEvents|InputActionJump
  (params (Key :type Key%20Structure :default "None"))
  (bind _charactermovement (Variables|Character|GetCharacterMovement))
  (bind _charactermovement_2 (Variables|Character|GetCharacterMovement))
  (bind _charactermovement_3 (Variables|Character|GetCharacterMovement))
  ;[1 1 1] Movemnet Controls
  (:Pressed
    (if (not (Variables|Default|GetJump%20CD%20is%20ON))
      (if (> (Variables|Default|GetSpeedOfCharacter) 0.5)
        (if (> (Variables|Default|GetSpeedOfCharacter) 2.5e+02)
          (Variables|/Script/Engine.CharacterMovementComponent|SetJumpZVelocity _charactermovement_2 5e+02)
          (else
            (Variables|/Script/Engine.CharacterMovementComponent|SetJumpZVelocity _charactermovement_2 4e+02)))
        (Character|Jump)
        (Variables|Default|SetJump%20CD%20is%20ON true)
        (Utilities|FlowControl|Delay 1.0)
        (Variables|Default|SetJump%20CD%20is%20ON false)
        (else
          (Variables|Default|SetJumped true)
          (Variables|/Script/Engine.CharacterMovementComponent|SetMaxWalkSpeed _charactermovement_3 0.0)
          (Variables|/Script/Engine.CharacterMovementComponent|SetbOrientRotationToMovement _charactermovement_3 false)
          (Utilities|FlowControl|Delay 1.65)
          (Variables|/Script/Engine.CharacterMovementComponent|SetMaxWalkSpeed _charactermovement 225.0)
          (Variables|/Script/Engine.CharacterMovementComponent|SetbOrientRotationToMovement _charactermovement true)
          (Variables|Default|SetJumped false)))))
  (:Released
    (Character|StopJumping)))

(event Input|ActionEvents|InputActionCameraDown
  (params (Key :type Key%20Structure :default "None"))
  ;[1 1 1] Camera Controls
  ;;[1 1 1] Camera Offset System
  (:Pressed
    (if (Utilities|Enum|Equal(Enum) (Variables|Default|GetDirection) "LeftSide")
      (Variables|/Script/Engine.SpringArmComponent|SetSocketOffset (Variables|Default|GetSpringArm) "-400.000000,0.000000,0.000000")
      (Variables|Default|SetSpeedOfVinterp 3.0)
      (elif (Utilities|Enum|Equal(Enum) (Variables|Default|GetDirection) "FrontSide")
        (Variables|/Script/Engine.SpringArmComponent|SetSocketOffset (Variables|Default|GetSpringArm1) "-400.000000,0.000000,0.000000")
        (Variables|Default|SetSpeedOfVinterp 3.0)
        (else
          (Variables|/Script/Engine.SpringArmComponent|SetSocketOffset (Variables|Default|GetSpringArm1) "-4000.000000,0.000000,0.000000")
          (Variables|Default|SetSpeedOfVinterp 3.0)))))
  (:Released
    (if (Utilities|Enum|Equal(Enum) (Variables|Default|GetDirection) "LeftSide")
      (Variables|/Script/Engine.SpringArmComponent|SetSocketOffset (Variables|Default|GetSpringArm) "0, 0, 0")
      (Variables|Default|SetSpeedOfVinterp 3.0)
      (elif (Utilities|Enum|Equal(Enum) (Variables|Default|GetDirection) "FrontSide")
        (Variables|/Script/Engine.SpringArmComponent|SetSocketOffset (Variables|Default|GetSpringArm1) "0, 0, 0")
        (Variables|Default|SetSpeedOfVinterp 3.0)
        (else
          (Variables|/Script/Engine.SpringArmComponent|SetSocketOffset (Variables|Default|GetSpringArm2) "0, 0, 0")
          (Variables|Default|SetSpeedOfVinterp 3.0))))))

(event Input|ActionEvents|InputActionCameraRight
  (params (Key :type Key%20Structure :default "None"))
  ;[1 1 1] Camera Controls
  ;;[1 1 1] Camera Offset System
  (:Pressed
    (if (Utilities|Enum|Equal(Enum) (Variables|Default|GetDirection) "LeftSide")
      (Variables|/Script/Engine.SpringArmComponent|SetSocketOffset (Variables|Default|GetSpringArm) "0,400.000000,0.000000")
      (Variables|Default|SetSpeedOfVinterp 3.0)
      (elif (Utilities|Enum|Equal(Enum) (Variables|Default|GetDirection) "FrontSide")
        (Variables|/Script/Engine.SpringArmComponent|SetSocketOffset (Variables|Default|GetSpringArm1) "0.000000,400.000000,0.000000")
        (Variables|Default|SetSpeedOfVinterp 3.0)
        (else
          (Variables|/Script/Engine.SpringArmComponent|SetSocketOffset (Variables|Default|GetSpringArm1) "0.000000,400.000000,0.000000")
          (Variables|Default|SetSpeedOfVinterp 3.0)))))
  (:Released
    (if (Utilities|Enum|Equal(Enum) (Variables|Default|GetDirection) "LeftSide")
      (Variables|/Script/Engine.SpringArmComponent|SetSocketOffset (Variables|Default|GetSpringArm) "0, 0, 0")
      (Variables|Default|SetSpeedOfVinterp 3.0)
      (elif (Utilities|Enum|Equal(Enum) (Variables|Default|GetDirection) "FrontSide")
        (Variables|/Script/Engine.SpringArmComponent|SetSocketOffset (Variables|Default|GetSpringArm1) "0, 0, 0")
        (Variables|Default|SetSpeedOfVinterp 3.0)
        (else
          (Variables|/Script/Engine.SpringArmComponent|SetSocketOffset (Variables|Default|GetSpringArm2) "0, 0, 0")
          (Variables|Default|SetSpeedOfVinterp 3.0))))))

(event Input|ActionEvents|InputActionCameraLeft
  (params (Key :type Key%20Structure :default "None"))
  ;[1 1 1] Camera Controls
  ;;[1 1 1] Camera Offset System
  (:Pressed
    (if (Utilities|Enum|Equal(Enum) (Variables|Default|GetDirection) "LeftSide")
      (Variables|/Script/Engine.SpringArmComponent|SetSocketOffset (Variables|Default|GetSpringArm) "0,-400.000000,0.000000")
      (Variables|Default|SetSpeedOfVinterp 3.0)
      (elif (Utilities|Enum|Equal(Enum) (Variables|Default|GetDirection) "FrontSide")
        (Variables|/Script/Engine.SpringArmComponent|SetSocketOffset (Variables|Default|GetSpringArm1) "0.000000,-400.000000,0.000000")
        (Variables|Default|SetSpeedOfVinterp 3.0)
        (else
          (Variables|/Script/Engine.SpringArmComponent|SetSocketOffset (Variables|Default|GetSpringArm1) "0.000000,-400.000000,0.000000")
          (Variables|Default|SetSpeedOfVinterp 3.0)))))
  (:Released
    (if (Utilities|Enum|Equal(Enum) (Variables|Default|GetDirection) "LeftSide")
      (Variables|/Script/Engine.SpringArmComponent|SetSocketOffset (Variables|Default|GetSpringArm) "0, 0, 0")
      (Variables|Default|SetSpeedOfVinterp 3.0)
      (elif (Utilities|Enum|Equal(Enum) (Variables|Default|GetDirection) "FrontSide")
        (Variables|/Script/Engine.SpringArmComponent|SetSocketOffset (Variables|Default|GetSpringArm1) "0, 0, 0")
        (Variables|Default|SetSpeedOfVinterp 3.0)
        (else
          (Variables|/Script/Engine.SpringArmComponent|SetSocketOffset (Variables|Default|GetSpringArm2) "0, 0, 0")
          (Variables|Default|SetSpeedOfVinterp 3.0))))))

(event Input|ActionEvents|InputActionCameraUP
  (params (Key :type Key%20Structure :default "None"))
  ;[1 1 1] Camera Controls
  ;;[1 1 1] Camera Offset System
  (:Pressed
    (if (Utilities|Enum|Equal(Enum) (Variables|Default|GetDirection) "LeftSide")
      (Variables|/Script/Engine.SpringArmComponent|SetSocketOffset (Variables|Default|GetSpringArm) "400.000000,0.000000,0.000000")
      (Variables|Default|SetSpeedOfVinterp 3.0)
      (elif (Utilities|Enum|Equal(Enum) (Variables|Default|GetDirection) "FrontSide")
        (Variables|/Script/Engine.SpringArmComponent|SetSocketOffset (Variables|Default|GetSpringArm1) "400.000000,0.000000,0.000000")
        (Variables|Default|SetSpeedOfVinterp 3.0)
        (else
          (Variables|/Script/Engine.SpringArmComponent|SetSocketOffset (Variables|Default|GetSpringArm1) "400.000000,400.000000,0.000000")
          (Variables|Default|SetSpeedOfVinterp 3.0)))))
  (:Released
    (if (Utilities|Enum|Equal(Enum) (Variables|Default|GetDirection) "LeftSide")
      (Variables|/Script/Engine.SpringArmComponent|SetSocketOffset (Variables|Default|GetSpringArm) "0, 0, 0")
      (Variables|Default|SetSpeedOfVinterp 3.0)
      (elif (Utilities|Enum|Equal(Enum) (Variables|Default|GetDirection) "FrontSide")
        (Variables|/Script/Engine.SpringArmComponent|SetSocketOffset (Variables|Default|GetSpringArm1) "0, 0, 0")
        (Variables|Default|SetSpeedOfVinterp 3.0)
        (else
          (Variables|/Script/Engine.SpringArmComponent|SetSocketOffset (Variables|Default|GetSpringArm2) "0, 0, 0")
          (Variables|Default|SetSpeedOfVinterp 3.0))))))

(event Input|AxisEvents|InputAxisMoveForward
  (params (AxisValue :type Float%20%28single-precision%29))
  ;[1 1 1] Movemnet Controls
  (Variables|Default|SetAxisValue AxisValue)
  (if (Utilities|Enum|Equal(Enum) (Variables|Default|GetDirection) "LeftSide")
    (Pawn|Input|AddMovementInput "0.000000,1.000000, 0" (Variables|Default|GetAxisValue) false)
    (elif (Utilities|Enum|Equal(Enum) (Variables|Default|GetDirection) "FrontSide")
      (Pawn|Input|AddMovementInput "1.000000,0.000000, 0" (Variables|Default|GetAxisValue) false)
      (else
        (Pawn|Input|AddMovementInput "0,-1.000000, 0" (Variables|Default|GetAxisValue) false)))))

(event Input|AxisEvents|InputAxisMoveRight
  (params (AxisValue :type Float%20%28single-precision%29))
  ;[1 1 1] Movemnet Controls
  (Variables|Default|SetAxisValue AxisValue)
  (if (Utilities|Enum|Equal(Enum) (Variables|Default|GetDirection) "LeftSide")
    (Pawn|Input|AddMovementInput "1.000000, 0, 0" (Variables|Default|GetAxisValue) false)
    (elif (Utilities|Enum|Equal(Enum) (Variables|Default|GetDirection) "FrontSide")
      (Pawn|Input|AddMovementInput "0,-1.000000, 0" (Variables|Default|GetAxisValue) false)
      (else
        (Pawn|Input|AddMovementInput "-1.000000,0.000000, 0" (Variables|Default|GetAxisValue) false)))))

(fn ConstructionScript)