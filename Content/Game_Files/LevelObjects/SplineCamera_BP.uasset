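; SplineCamera_BP is a trigger-box camera zone that glides the player's SplineCamera along a spline as the player moves.
; Entering the Box blends the view to that camera, and Tick interpolates it toward the spline point closest to the player.
; The active Box grows slightly as an exit margin.
; Overlapping zones hand off via LastUsedSplineCamera and ShouldReset, and leaving all zones blends back to ActiveCamera.
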(event OnComponentBeginOverlap(Box)
  (params (OverlappedComponent :type Primitive%20Component%20Object%20Reference) (OtherActor :type Actor%20Object%20Reference) (OtherComp :type Primitive%20Component%20Object%20Reference) (OtherBodyIndex :type Integer) (bFromSweep :type Boolean) (SweepResult :type Hit%20Result%20Structure%20%28by%20ref%29))
  (bind _asmain_character_bp (Utilities|Casting|CastToMainCharacterBP OtherActor))
  (if (Variables|/Game/Game_Files/Characters/Main_Character/MainCharacterBP.MainCharacterBP_C|GetIsOverlapingSplineCamera _asmain_character_bp)
    (Variables|SplineCamera_BP_C|SetIsActive (Variables|/Game/Game_Files/Characters/Main_Character/MainCharacterBP.MainCharacterBP_C|GetLastUsedSplineCamera (Variables|Default|GetPlayer)) false)
    (Variables|SplineCamera_BP_C|SetShouldReset (Variables|/Game/Game_Files/Characters/Main_Character/MainCharacterBP.MainCharacterBP_C|GetLastUsedSplineCamera (Variables|Default|GetPlayer)) false)
    (CallFunction|StopUsing (Variables|/Game/Game_Files/Characters/Main_Character/MainCharacterBP.MainCharacterBP_C|GetLastUsedSplineCamera (Variables|Default|GetPlayer)))
    (Variables|Default|SetIsActive true)
    (bind _output_get (Variables|Default|SetDefaultScale (Transformation|GetWorldScale (Variables|Default|GetBox))))
    (Transformation|SetWorldScale3D (Variables|Default|GetBox) (* _output_get 1.1))
    (Variables|/Game/Game_Files/Characters/Main_Character/MainCharacterBP.MainCharacterBP_C|SetLastUsedSplineCamera (Variables|Default|GetPlayer) self)
    (Variables|Default|SetShouldReset true)
    (else
      (Variables|/Game/Game_Files/Characters/Main_Character/MainCharacterBP.MainCharacterBP_C|SetIsOverlapingSplineCamera _asmain_character_bp true)
      (Variables|/Game/Game_Files/Characters/Main_Character/MainCharacterBP.MainCharacterBP_C|SetLastUsedSplineCamera (Variables|Default|GetPlayer) self)
      (Transformation|SetActorLocation (Variables|/Game/Game_Files/Characters/Main_Character/MainCharacterBP.MainCharacterBP_C|GetSplineCamera _asmain_character_bp) (Spline|FindLocationClosesttoWorldLocation (Variables|Default|GetSpline) (Transformation|GetActorLocation (Variables|Default|GetPlayer)) "World") false false)
      (Variables|Default|SetIsActive true)
      (Game|Player|SetViewTargetwithBlend (Game|GetPlayerController 0) (Variables|/Game/Game_Files/Characters/Main_Character/MainCharacterBP.MainCharacterBP_C|GetSplineCamera _asmain_character_bp) 1.0 "VTBlend_Linear" 0.0 true)
      (bind _output_get_2 (Variables|Default|SetDefaultScale (Transformation|GetWorldScale (Variables|Default|GetBox))))
      (Transformation|SetWorldScale3D (Variables|Default|GetBox) (* _output_get_2 1.1)))))

(event OnComponentEndOverlap(Box)
  (params (OverlappedComponent :type Primitive%20Component%20Object%20Reference) (OtherActor :type Actor%20Object%20Reference) (OtherComp :type Primitive%20Component%20Object%20Reference) (OtherBodyIndex :type Integer))
  (bind _player (Variables|Default|GetPlayer))
  (if (Variables|Default|GetShouldReset)
    (bind _outactors (Actor|GetAllActorsOfClass "SplineCamera_BP_C"))
    (for _array_element _outactors
      (if (Collision|IsOverlappingActor (Variables|Default|GetPlayer) _array_element :!class /Script/Engine.Actor)
        (Variables|Default|SetIsOverlapingAnotherSplineCamera true)
        (Variables|Default|SetAnotherSplineCameraOverlapingByPlayer _array_element)))
    (if (Variables|Default|GetIsOverlapingAnotherSplineCamera)
      (Development|PrintString (Utilities|GetDisplayName (Variables|Default|GetAnotherSplineCameraOverlapingByPlayer)) true true "(R=1.000000,G=0.034397,B=0.000000,A=1.000000)" 2e+01)
      (CallFunction|StartUsing (Variables|Default|GetAnotherSplineCameraOverlapingByPlayer))
      (Variables|Default|SetIsOverlapingAnotherSplineCamera false)
      (else
        (Utilities|Casting|CastToMainCharacterBP OtherActor)
        (Variables|Default|SetIsActive false)
        (Variables|/Game/Game_Files/Characters/Main_Character/MainCharacterBP.MainCharacterBP_C|SetIsOverlapingSplineCamera _player false)
        (Game|Player|SetViewTargetwithBlend (Game|GetPlayerController 0) (Variables|/Game/Game_Files/Characters/Main_Character/MainCharacterBP.MainCharacterBP_C|GetActiveCamera _player) 1.0 "VTBlend_Linear" 0.0 true)
        (Transformation|SetWorldScale3D (Variables|Default|GetBox) (Variables|Default|GetDefaultScale))))
    (else
      (Development|PrintString "False reset")
      (Variables|Default|SetShouldReset true))))

(event Custom|StopUsing
  (Transformation|SetWorldScale3D (Variables|Default|GetBox) (Variables|Default|GetDefaultScale)))

(event Custom|StartUsing
  (bind _asmain_character_bp (Utilities|Casting|CastToMainCharacterBP (stale OnComponentBeginOverlap(Box) OtherActor)))
  (if (Variables|/Game/Game_Files/Characters/Main_Character/MainCharacterBP.MainCharacterBP_C|GetIsOverlapingSplineCamera _asmain_character_bp)
    (Variables|SplineCamera_BP_C|SetIsActive (Variables|/Game/Game_Files/Characters/Main_Character/MainCharacterBP.MainCharacterBP_C|GetLastUsedSplineCamera (Variables|Default|GetPlayer)) false)
    (Variables|SplineCamera_BP_C|SetShouldReset (Variables|/Game/Game_Files/Characters/Main_Character/MainCharacterBP.MainCharacterBP_C|GetLastUsedSplineCamera (Variables|Default|GetPlayer)) false)
    (CallFunction|StopUsing (Variables|/Game/Game_Files/Characters/Main_Character/MainCharacterBP.MainCharacterBP_C|GetLastUsedSplineCamera (Variables|Default|GetPlayer)))
    (Variables|Default|SetIsActive true)
    (bind _output_get (Variables|Default|SetDefaultScale (Transformation|GetWorldScale (Variables|Default|GetBox))))
    (Transformation|SetWorldScale3D (Variables|Default|GetBox) (* _output_get 1.1))
    (Variables|/Game/Game_Files/Characters/Main_Character/MainCharacterBP.MainCharacterBP_C|SetLastUsedSplineCamera (Variables|Default|GetPlayer) self)
    (Variables|Default|SetShouldReset true)
    (else
      (Variables|/Game/Game_Files/Characters/Main_Character/MainCharacterBP.MainCharacterBP_C|SetIsOverlapingSplineCamera _asmain_character_bp true)
      (Variables|/Game/Game_Files/Characters/Main_Character/MainCharacterBP.MainCharacterBP_C|SetLastUsedSplineCamera (Variables|Default|GetPlayer) self)
      (Transformation|SetActorLocation (Variables|/Game/Game_Files/Characters/Main_Character/MainCharacterBP.MainCharacterBP_C|GetSplineCamera _asmain_character_bp) (Spline|FindLocationClosesttoWorldLocation (Variables|Default|GetSpline) (Transformation|GetActorLocation (Variables|Default|GetPlayer)) "World") false false)
      (Variables|Default|SetIsActive true)
      (Game|Player|SetViewTargetwithBlend (Game|GetPlayerController 0) (Variables|/Game/Game_Files/Characters/Main_Character/MainCharacterBP.MainCharacterBP_C|GetSplineCamera _asmain_character_bp) 1.0 "VTBlend_Linear" 0.0 true)
      (bind _output_get_2 (Variables|Default|SetDefaultScale (Transformation|GetWorldScale (Variables|Default|GetBox))))
      (Transformation|SetWorldScale3D (Variables|Default|GetBox) (* _output_get_2 1.1)))))

(event EventBeginPlay
  (bind _asmain_character_bp (Utilities|Casting|CastToMainCharacterBP (Game|GetPlayerCharacter 0)))
  (Variables|Default|SetPlayer _asmain_character_bp)
  (Variables|Default|SetShouldReset true))

(event EventTick
  (params (DeltaSeconds :type Float%20%28single-precision%29))
  (bind _player (Variables|Default|GetPlayer))
  (bind _splinecamera (Variables|/Game/Game_Files/Characters/Main_Character/MainCharacterBP.MainCharacterBP_C|GetSplineCamera _player))
  (if (Variables|Default|GetIsActive)
    (bind _output_get (Variables|Default|SetDelta%20Seconds DeltaSeconds))
    (bind _output_get_2 (Variables|Default|SetCurrentCameraLocation (Transformation|GetActorLocation _splinecamera)))
    (Transformation|SetActorLocation _splinecamera (Math|Interpolation|VInterpTo _output_get_2 (Spline|FindLocationClosesttoWorldLocation (Variables|Default|GetSpline) (Transformation|GetActorLocation (Variables|Default|GetPlayer)) "World") _output_get 2.0) false false)))

(fn ConstructionScript)