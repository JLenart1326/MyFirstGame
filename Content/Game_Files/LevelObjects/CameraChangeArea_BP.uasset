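; Level trigger volume that switches the player's view to a linked StaticCamera_BP and changes the character's CameraDirection.
; The construction script links the camera by matching Id and prints the result.
; Leaving restores the saved direction and the player's active camera.
; When areas overlap, the new one inherits the original direction, suppresses the previous area's exit reset and lowers that box below the player's feet, with no code raising it again.
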(event OnComponentBeginOverlap(Box)
  (params (OverlappedComponent :type Primitive%20Component%20Object%20Reference) (OtherActor :type Actor%20Object%20Reference) (OtherComp :type Primitive%20Component%20Object%20Reference) (OtherBodyIndex :type Integer) (bFromSweep :type Boolean) (SweepResult :type Hit%20Result%20Structure%20%28by%20ref%29))
  (bind _asmain_character_bp (Utilities|Casting|CastToMainCharacterBP OtherActor))
  (bind _output_get (Variables|Default|SetPlayer _asmain_character_bp))
  (Variables|Default|SetPlayerFeetZLocation (- (.z (Transformation|GetActorLocation (Variables|Default|GetPlayer))) (Components|Capsule|GetScaledCapsuleHalfHeight (Variables|/Script/Engine.Character|GetCapsuleComponent (Variables|Default|GetPlayer)))))
  (if (Variables|/Game/Game_Files/Characters/Main_Character/MainCharacterBP.MainCharacterBP_C|GetIsOverlappingWithCameraChanger _output_get)
    (Variables|CameraChangeArea_BP_C|SetCanEndOverlap (Variables|/Game/Game_Files/Characters/Main_Character/MainCharacterBP.MainCharacterBP_C|GetCurrentCameraChanger (Variables|Default|GetPlayer)) false)
    (Transformation|SetWorldLocation (Variables|CameraChangeArea_BP_C|GetBox (Variables|/Game/Game_Files/Characters/Main_Character/MainCharacterBP.MainCharacterBP_C|GetCurrentCameraChanger (Variables|Default|GetPlayer))) (Math|Vector|MakeVector (.x (Transformation|GetWorldLocation (Variables|CameraChangeArea_BP_C|GetBox (Variables|/Game/Game_Files/Characters/Main_Character/MainCharacterBP.MainCharacterBP_C|GetCurrentCameraChanger (Variables|Default|GetPlayer))))) (.y (Transformation|GetWorldLocation (Variables|CameraChangeArea_BP_C|GetBox (Variables|/Game/Game_Files/Characters/Main_Character/MainCharacterBP.MainCharacterBP_C|GetCurrentCameraChanger (Variables|Default|GetPlayer))))) (- (.z (Transformation|GetWorldLocation (Variables|CameraChangeArea_BP_C|GetBox (Variables|/Game/Game_Files/Characters/Main_Character/MainCharacterBP.MainCharacterBP_C|GetCurrentCameraChanger (Variables|Default|GetPlayer))))) (- (Variables|CameraChangeArea_BP_C|GetBoxTopBorderLocation (Variables|/Game/Game_Files/Characters/Main_Character/MainCharacterBP.MainCharacterBP_C|GetCurrentCameraChanger (Variables|Default|GetPlayer))) (- (Variables|Default|GetPlayerFeetZLocation) 5.0)))) false false)
    (Variables|Default|SetOldDirection (Variables|CameraChangeArea_BP_C|GetOldDirection (Variables|/Game/Game_Files/Characters/Main_Character/MainCharacterBP.MainCharacterBP_C|GetCurrentCameraChanger (Variables|Default|GetPlayer))))
    (else
      (Variables|/Game/Game_Files/Characters/Main_Character/MainCharacterBP.MainCharacterBP_C|SetIsOverlappingWithCameraChanger (Variables|Default|GetPlayer) true)
      (Variables|Default|SetOldDirection (Variables|/Game/Game_Files/Characters/Main_Character/MainCharacterBP.MainCharacterBP_C|GetCameraDirection (Variables|Default|GetPlayer)))))
  (Variables|/Game/Game_Files/Characters/Main_Character/MainCharacterBP.MainCharacterBP_C|SetCurrentCameraChanger (Variables|Default|GetPlayer) self)
  (Variables|Default|SetCanEndOverlap true)
  (Variables|/Game/Game_Files/Characters/Main_Character/MainCharacterBP.MainCharacterBP_C|SetCameraDirection (Variables|Default|GetPlayer) (Variables|Default|GetNewDirection))
  (Game|Player|SetViewTargetwithBlend (Game|GetPlayerController 0) (Variables|Default|GetConnectedCamera) 0.0 "VTBlend_Linear" 0.0 false))

(event OnComponentEndOverlap(Box)
  (params (OverlappedComponent :type Primitive%20Component%20Object%20Reference) (OtherActor :type Actor%20Object%20Reference) (OtherComp :type Primitive%20Component%20Object%20Reference) (OtherBodyIndex :type Integer))
  (bind _player (Variables|Default|GetPlayer))
  (if (Variables|Default|GetCanEndOverlap)
    (Variables|/Game/Game_Files/Characters/Main_Character/MainCharacterBP.MainCharacterBP_C|SetCameraDirection _player (Variables|Default|GetOldDirection))
    (Game|Player|SetViewTargetwithBlend (Game|GetPlayerController 0) (Variables|/Game/Game_Files/Characters/Main_Character/MainCharacterBP.MainCharacterBP_C|GetActiveCamera _player) 0.0 "VTBlend_Linear" 0.0 false)
    (Variables|/Game/Game_Files/Characters/Main_Character/MainCharacterBP.MainCharacterBP_C|SetIsOverlappingWithCameraChanger (Variables|Default|GetPlayer) false)))

(event EventBeginPlay
  (bind _box (Variables|Default|GetBox))
  (bind _box_2 (Variables|Default|GetBox))
  (bind _returnvalue (Transformation|GetWorldScale _box_2))
  (bind _boxextent (Variables|/Script/Engine.BoxComponent|GetBoxExtent _box))
  (Variables|Default|SetBoxTopBorderLocation (+ (/ (.z (Math|Vector|MakeVector (* (* 2 (.x _boxextent)) (.x _returnvalue)) (* (* 2 (.y _boxextent)) (.y _returnvalue)) (* (* 2 (.z _boxextent)) (.z _returnvalue)))) 2.0) (.z (Transformation|GetWorldLocation (Variables|Default|GetBox))))))

(fn ConstructionScript
  (bind _outactors (Actor|GetAllActorsOfClass "/Game/Game_Files/LevelObjects/StaticCamera_BP.StaticCamera_BP_C"))
  (for _array_element _outactors
    (if (== (Variables|/Game/Game_Files/LevelObjects/StaticCamera_BP.StaticCamera_BP_C|GetId _array_element) (Variables|Default|GetId))
      (Variables|Default|SetConnectedCamera _array_element)))
  (if (== (Variables|Default|GetConnectedCamera) 0)
    (Development|PrintString "Brak podłączonej kamery")
    (else
      (Development|PrintString (Utilities|GetDisplayName (Variables|Default|GetConnectedCamera))))))