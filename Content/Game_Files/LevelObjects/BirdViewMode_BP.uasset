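; BirdViewMode_BP is a box trigger volume that lets the main character use bird view mode while inside it.
; On entry, the first volume sets the player's bird-view flags and shows a ChangeToBirdViewNotify widget.
; When that volume is exited, it removes the widget and searches all instances for another overlapped one to take over via BeginOverlap.
; If none is found, it disables bird mode and switches bird view off.
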(event OnComponentBeginOverlap(Box)
  (params (OverlappedComponent :type Primitive%20Component%20Object%20Reference) (OtherActor :type Actor%20Object%20Reference) (OtherComp :type Primitive%20Component%20Object%20Reference) (OtherBodyIndex :type Integer) (bFromSweep :type Boolean) (SweepResult :type Hit%20Result%20Structure%20%28by%20ref%29))
  (bind _asmain_character_bp (Utilities|Casting|CastToMainCharacterBP OtherActor))
  (bind _output_get (Variables|Default|SetPlayer _asmain_character_bp))
  (if (not (Variables|/Game/Game_Files/Characters/Main_Character/MainCharacterBP.MainCharacterBP_C|GetIsOverlappingWithBirdView _output_get))
    (Variables|/Game/Game_Files/Characters/Main_Character/MainCharacterBP.MainCharacterBP_C|SetIsOverlappingWithBirdView _output_get true)
    (Variables|/Game/Game_Files/Characters/Main_Character/MainCharacterBP.MainCharacterBP_C|SetCanUseBirdMode _output_get true)
    (Variables|Default|GetWidget
      (:then)
      (:else
        (bind _returnvalue (UserInterface|CreateWidget "/Game/Game_Files/Characters/Main_Character/UserInterface/ChangeToBirdViewNotify.ChangeToBirdViewNotify_C"))
        (bind _output_get_2 (Variables|Default|SetWidget _returnvalue))
        (UserInterface|Viewport|AddtoViewport _output_get_2 0)))))

(event OnComponentEndOverlap(Box)
  (params (OverlappedComponent :type Primitive%20Component%20Object%20Reference) (OtherActor :type Actor%20Object%20Reference) (OtherComp :type Primitive%20Component%20Object%20Reference) (OtherBodyIndex :type Integer))
  (bind _asmain_character_bp (Utilities|Casting|CastToMainCharacterBP OtherActor))
  (Variables|Default|SetPlayer _asmain_character_bp)
  (bind _widget (Variables|Default|GetWidget)
    (:then
      (Widget|RemovefromParent _widget)
      (Variables|Default|SetWidget 0)
      (bind _outactors (Actor|GetAllActorsOfClass "BirdViewMode_BP_C"))
      (bind _array_element (Utilities|Array|ForEachLoopwithBreak _outactors :!label _label)
        (:LoopBody
          (if (Collision|IsOverlappingActor (Variables|Default|GetPlayer) _array_element :!class /Script/Engine.Actor)
            (Variables|Default|SetIsOverlaping%20AnotherBirdViewMode true)
            (bind _output_get (Variables|Default|SetAnotherBirdView _array_element))
            (Variables|BirdViewMode_BP_C|SetLastBirdViewMode _output_get self)
            (goto _label Break)
            (else
              (Variables|Default|SetIsOverlaping%20AnotherBirdViewMode false))))
        (:Completed
          (if (Variables|Default|GetIsOverlaping%20AnotherBirdViewMode)
            (CallFunction|BeginOverlap (Variables|Default|GetAnotherBirdView))
            (else
              (Variables|/Game/Game_Files/Characters/Main_Character/MainCharacterBP.MainCharacterBP_C|SetCanUseBirdMode (Variables|Default|GetPlayer) false)
              (if (Variables|/Game/Game_Files/Characters/Main_Character/MainCharacterBP.MainCharacterBP_C|GetBirdViewOn? (Variables|Default|GetPlayer))
                (Variables|/Game/Game_Files/Characters/Main_Character/MainCharacterBP.MainCharacterBP_C|SetBirdViewOn? (Variables|Default|GetPlayer) false))
              (Variables|/Game/Game_Files/Characters/Main_Character/MainCharacterBP.MainCharacterBP_C|SetIsOverlappingWithBirdView (Variables|Default|GetPlayer) false))))))
    (:else)))

(event Custom|BeginOverlap
  (Variables|/Game/Game_Files/Characters/Main_Character/MainCharacterBP.MainCharacterBP_C|SetIsOverlappingWithBirdView (Variables|Default|GetPlayer) false)
  (bind _asmain_character_bp (Utilities|Casting|CastToMainCharacterBP (stale OnComponentBeginOverlap(Box) OtherActor)))
  (bind _output_get (Variables|Default|SetPlayer _asmain_character_bp))
  (if (not (Variables|/Game/Game_Files/Characters/Main_Character/MainCharacterBP.MainCharacterBP_C|GetIsOverlappingWithBirdView _output_get))
    (Variables|/Game/Game_Files/Characters/Main_Character/MainCharacterBP.MainCharacterBP_C|SetIsOverlappingWithBirdView _output_get true)
    (Variables|/Game/Game_Files/Characters/Main_Character/MainCharacterBP.MainCharacterBP_C|SetCanUseBirdMode _output_get true)
    (Variables|Default|GetWidget
      (:then)
      (:else
        (bind _returnvalue (UserInterface|CreateWidget "/Game/Game_Files/Characters/Main_Character/UserInterface/ChangeToBirdViewNotify.ChangeToBirdViewNotify_C"))
        (bind _output_get_2 (Variables|Default|SetWidget _returnvalue))
        (UserInterface|Viewport|AddtoViewport _output_get_2 0)))))

(fn ConstructionScript)