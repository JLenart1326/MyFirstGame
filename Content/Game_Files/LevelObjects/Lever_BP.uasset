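; Interactable lever that plays an assigned level sequence forward or in reverse on alternate pulls.
; BeginPlay creates the sequence player and opens or closes an interaction gate based on whether ConnectedObject is valid, printing Polish debug messages.
; Interaction plays the player's pulling montage and locks movement during a delay, then a flip-flopped timeline rotates the rod.
; Each timeline finish flip-flops the sequence direction; ConnectedObject is only validity-checked.
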(event EventBeginPlay
  (bind _connectedlevelsequence (Variables|Default|GetConnectedLevelSequence))
  (bind _player (Variables|Default|GetPlayer))
  (Utilities|IsValid _connectedlevelsequence
    (:Is%20Valid
      (bind _returnvalue (Sequencer|Player|CreateLevelSequencePlayer _connectedlevelsequence))
      (Variables|Default|SetLevelSequencePlayer _returnvalue)
      (Utilities|IsValid (Variables|Default|GetConnectedObject)
        (:Is%20Valid
          (Utilities|FlowControl|Gate true) ; enters at Open
        )
        (:Is%20Not%20Valid
          (Development|PrintString "Nie podpiety objekt")
          (Utilities|FlowControl|Gate true) ; enters at Close
        )))
    (:Is%20Not%20Valid
      (Development|PrintString "Nie podpiety LS"))))

(event EventOnInteracted
  (params (Player :type Main%20Character%20BP%20Object%20Reference) (Interacter :type Actor%20Object%20Reference) (IsUsingGamepad :type Boolean))
  (bind _levelsequenceplayer (Variables|Default|GetLevelSequencePlayer))
  (Variables|Default|SetPlayer Player)
  (Utilities|FlowControl|Gate true
    (:Exit
      (Development|PrintString (Utilities|String|Append "Pomyslnie wyslano wiadomosc z interfejsu obiektu: " (Utilities|String|MakeLiteralString (Utilities|GetDisplayName self)) ".   Wszystko działa poprawnie!"))
      (Animation|PlayAnimMontage (Variables|Default|GetPlayer) "/Game/Game_Files/Characters/Main_Character/Animations/Pulling_Lever_Montage.Pulling_Lever_Montage" 1.0 "None")
      (Variables|/Game/Game_Files/Characters/Main_Character/MainCharacterBP.MainCharacterBP_C|SetCan%20move? (Variables|Default|GetPlayer) false)
      (Utilities|FlowControl|Delay 2.0)
      (Variables|/Game/Game_Files/Characters/Main_Character/MainCharacterBP.MainCharacterBP_C|SetCan%20move? (Variables|Default|GetPlayer) true)
      (Utilities|FlowControl|FlipFlop
        (:A
          (bind _leverpull (Timeline|PullTheLever Play)
            (:Update
              (Transformation|SetRelativeRotation (Variables|Default|GetRod) (Math|Rotator|MakeRotator 0.0 0.0 _leverpull) false false))
            (:Finished
              (Utilities|FlowControl|FlipFlop
                (:A
                  (Sequencer|Player|Play _levelsequenceplayer :!class /Script/MovieScene.MovieSceneSequencePlayer))
                (:B
                  (Class|MovieSceneSequencePlayer|PlayReverse _levelsequenceplayer))))))
        (:B
          (Timeline|PullTheLever Reverse))))))

(fn ConstructionScript)