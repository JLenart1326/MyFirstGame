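; Climbable ladder actor that the main character can mount, climb and leave at the top.
; Construction script stacks mesh segments from LadderHeight, sizing and placing the trigger boxes, climb transforms and end position to match.
; Main box overlap flags the character as near the ladder; the top box plays a climb-up montage with input locked, then restores walking after a delay.
; Helper functions find the nearest climb transform and move the character to the end position.
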(event OnComponentBeginOverlap(Box)
  (params (OverlappedComponent :type Primitive%20Component%20Object%20Reference) (OtherActor :type Actor%20Object%20Reference) (OtherComp :type Primitive%20Component%20Object%20Reference) (OtherBodyIndex :type Integer) (bFromSweep :type Boolean) (SweepResult :type Hit%20Result%20Structure%20%28by%20ref%29))
  (bind _asmain_character_bp (Utilities|Casting|CastToMainCharacterBP OtherActor))
  (Variables|/Game/Game_Files/Characters/Main_Character/MainCharacterBP.MainCharacterBP_C|SetNearTheLadder? _asmain_character_bp true)
  (Variables|/Game/Game_Files/Characters/Main_Character/MainCharacterBP.MainCharacterBP_C|SetOverlapedLadderActor _asmain_character_bp self))

(event OnComponentEndOverlap(Box)
  (params (OverlappedComponent :type Primitive%20Component%20Object%20Reference) (OtherActor :type Actor%20Object%20Reference) (OtherComp :type Primitive%20Component%20Object%20Reference) (OtherBodyIndex :type Integer))
  (bind _asmain_character_bp (Utilities|Casting|CastToMainCharacterBP OtherActor))
  (Variables|/Game/Game_Files/Characters/Main_Character/MainCharacterBP.MainCharacterBP_C|SetNearTheLadder? _asmain_character_bp false)
  (Utilities|FlowControl|DoOnce false
    (:Completed
      (Pawn|Components|CharacterMovement|SetMovementMode (Variables|/Script/Engine.Character|GetCharacterMovement _asmain_character_bp) "MOVE_Walking" 0)
      (Variables|/Game/Game_Files/Characters/Main_Character/MainCharacterBP.MainCharacterBP_C|SetOnLadder? _asmain_character_bp false)
      (Variables|/Game/Game_Files/Characters/Main_Character/MainCharacterBP.MainCharacterBP_C|SetOverlapedLadderActor _asmain_character_bp 0))))

(event OnComponentBeginOverlap(EndClimbingBox)
  (params (OverlappedComponent :type Primitive%20Component%20Object%20Reference) (OtherActor :type Actor%20Object%20Reference) (OtherComp :type Primitive%20Component%20Object%20Reference) (OtherBodyIndex :type Integer) (bFromSweep :type Boolean) (SweepResult :type Hit%20Result%20Structure%20%28by%20ref%29))
  (bind _asmain_character_bp (Utilities|Casting|CastToMainCharacterBP OtherActor))
  (if (Variables|/Game/Game_Files/Characters/Main_Character/MainCharacterBP.MainCharacterBP_C|GetOnLadder? _asmain_character_bp)
    (Input|DisableInput _asmain_character_bp 0)
    (Variables|/Game/Game_Files/Characters/Main_Character/MainCharacterBP.MainCharacterBP_C|SetCan%20move? _asmain_character_bp false)
    (Variables|/Game/Game_Files/Characters/Main_Character/MainCharacterBP.MainCharacterBP_C|SetOnLadder? _asmain_character_bp false)
    (Animation|PlayAnimMontage _asmain_character_bp "/Game/Game_Files/Characters/Main_Character/Animations/Climbing_To_Top_Montage.Climbing_To_Top_Montage" 1.0 "None")
    (Utilities|FlowControl|Delay 3.0)
    (Input|EnableInput _asmain_character_bp 0)
    (Variables|/Game/Game_Files/Characters/Main_Character/MainCharacterBP.MainCharacterBP_C|SetCan%20move? _asmain_character_bp true)
    (Pawn|Components|CharacterMovement|SetMovementMode (Variables|/Script/Engine.Character|GetCharacterMovement _asmain_character_bp) "MOVE_Walking" 0)
    (else
      (Development|PrintString "Nie wspinasz sie"))))

(event OnComponentEndOverlap(EndClimbingBox)
  (params (OverlappedComponent :type Primitive%20Component%20Object%20Reference) (OtherActor :type Actor%20Object%20Reference) (OtherComp :type Primitive%20Component%20Object%20Reference) (OtherBodyIndex :type Integer))
  (Utilities|Casting|CastToMainCharacterBP OtherActor))

(event Custom|Reset%20movement%20change
  (Utilities|FlowControl|DoOnce false) ; enters at Reset
)

(fn ConstructionScript
  (bind _ladderheight (Variables|Default|GetLadderHeight))
  (bind _ladderbase (Variables|Default|GetLadderBase))
  (bind _ladderbase_2 (Variables|Default|GetLadderBase))
  (bind _ladderheight_2 (Variables|Default|GetLadderHeight))
  (bind _returnvalue (/ _ladderheight 6e+01))
  (bind _returnvalue_2 (Transformation|GetRelativeTransform _ladderbase_2))
  (bind _returnvalue_3 (/ _ladderheight_2 6e+01))
  (bind _returnvalue_4 (Transformation|GetRelativeTransform _ladderbase))
  (bind _returnvalue_5 (Math|Float|Truncate _returnvalue_3))
  (bind _returnvalue_6 (Math|Float|Truncate _returnvalue))
  (bind _returnvalue_7 (+ _returnvalue_5 1))
  (bind _returnvalue_8 (+ _returnvalue_6 1))
  (for _array_element (Variables|Default|GetPositionTransforms)
    (AddComponent|AddArrowComponent false _array_element))
  (for _index (range 0 _returnvalue_8)
    (bind _returnvalue_9 (AddComponent|AddStaticMeshComponent false (Math|Transform|MakeTransform (Math|Vector|MakeVector (.x (.location _returnvalue_2)) (.y (.location _returnvalue_2)) (+ (* _index 37.0) 55.0)) (.rotation _returnvalue_2) (.scale _returnvalue_2))))
    (Collision|SetCollisionObjectType _returnvalue_9 "ECC_GameTraceChannel3"))
  (bind _returnvalue_10 (AddComponent|AddStaticMeshComponent false (Math|Transform|MakeTransform (Math|Vector|MakeVector (.x (.location _returnvalue_4)) (.y (.location _returnvalue_4)) (+ (+ (* _returnvalue_8 37.0) 55.0) 37.0)) (.rotation _returnvalue_4) (.scale _returnvalue_4))))
  (Collision|SetCollisionObjectType _returnvalue_10 "ECC_GameTraceChannel3")
  (Collision|SetCollisionResponsetoAllChannels _returnvalue_9 "ECR_Ignore")
  (Variables|Default|SetPositionTransforms (Utilities|Array|MakeArray (Math|Transform|MakeTransform "22.646214,20.000000,43.815384" "0.000000,-90.000343, 0") (Math|Transform|MakeTransform (Math|Vector|MakeVector 22.646214 2e+01 (+ 105.600006 (* _returnvalue_7 37.0))) "0,-90.000343, 0")))
  (Variables|Default|SetEndPosition (Math|Transform|MakeTransform (Math|Vector|MakeVector 22.646116 -19.200256 (+ (* _returnvalue_7 37.0) 197.0))))
  (Transformation|SetRelativeLocation (Variables|Default|GetEndClimbingBox) (Math|Vector|MakeVector 24.999886 30.000151 (+ (* _returnvalue_5 37.0) 1.6e+02)) false false)
  (Transformation|SetRelativeScale3D (Variables|Default|GetBox) (Math|Vector|MakeVector 1.0 1.0 (+ (* _returnvalue_7 1.0) 2.9375)))
  (Transformation|SetRelativeLocation (Variables|Default|GetBox) (Math|Vector|MakeVector 23.0 -9.0 (+ (* _returnvalue_7 5.0) 75.0)) false false))

(fn FindClosestClimbIndex
  (params (CharacterLocation :type Vector))
  (for (_array_element _array_index) (Variables|Default|GetPositionTransforms)
    (LocalVariables|SetCurrentTransformIndex _array_index)
    (LocalVariables|SetTheCurrentDistance (Class|KismetMathLibrary|VectorDistanceSquared (Math|Transform|TransformLocation (Transformation|GetActorTransform) (.location _array_element)) CharacterLocation))
    (if (<= (LocalVariables|GetCurrentTransformIndex) 0)
      (LocalVariables|SetClosestTransformIIndex (LocalVariables|GetCurrentTransformIndex) :!label _label)
      (LocalVariables|SetTheClosestDistance (LocalVariables|GetTheCurrentDistance))
      (elif (< (LocalVariables|GetTheCurrentDistance) (LocalVariables|GetTheClosestDistance))
        (goto _label))))
  (return (LocalVariables|GetClosestTransformIIndex)))

(fn SetCharacterinCorrectPosition
  (params (Character :type Main%20Character%20BP%20Object%20Reference))
  (bind _output_get (LocalVariables|SetClimbingCharacter Character))
  (Variables|/Game/Game_Files/Characters/Main_Character/MainCharacterBP.MainCharacterBP_C|SetOnLadder? _output_get false)
  (Transformation|SetActorLocation (LocalVariables|GetClimbingCharacter) (Math|Transform|TransformLocation (Transformation|GetActorTransform) (.location (Variables|Default|GetEndPosition))) false false))