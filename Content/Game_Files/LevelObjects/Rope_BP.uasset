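; Interactable swing rope that the player hangs from, swings on and launches off.
; Construction sizes the cable end and capsule from RopeLength.
; Physics constraints link start, a runtime joint and end, drawn by two cables; interaction rebuilds the joint at the player's height, attaches them and pushes it using their prior speed and facing.
; LaunchPlayer passes the joint's velocity to the character and briefly switches the capsule's collision type.
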(event Custom|Add%20swinging%20force
  (params (Swing%20force :type Vector) (Axis%20value :type Float%20%28single-precision%29))
  (Physics|AddForce (Variables|Default|GetJoint) (* (* Swing%20force Axis%20value) 1.8e+02) "None" true))

(event Custom|LaunchPlayer
  (bind _player (Variables|Default|GetPlayer))
  (bind _capsule (Variables|Default|GetCapsule))
  (bind _player_2 (Variables|Default|GetPlayer))
  (bind _returnvalue (Transformation|GetActorRotation _player))
  (Transformation|DetachFromActor _player_2 "KeepWorld" "KeepWorld" "KeepWorld")
  (Transformation|SetActorRotation _player_2 (Math|Rotator|MakeRotator 0.0 0.0 (.yaw (Transformation|GetActorRotation _player_2))))
  (bind _returnvalue_2 (Physics|GetPhysicsLinearVelocity (Variables|Default|GetJoint) "None"))
  (Character|LaunchCharacter _player (* _returnvalue_2 1.0) false false)
  (Transformation|SetActorRotation _player (Math|Rotator|MakeRotator (.roll _returnvalue) (.pitch _returnvalue) (.yaw (Math|Rotator|MakeRotfromX _returnvalue_2))))
  (Variables|/Game/Game_Files/Characters/Main_Character/MainCharacterBP.MainCharacterBP_C|SetRope _player 0)
  (Variables|/Game/Game_Files/Characters/Main_Character/MainCharacterBP.MainCharacterBP_C|SetIsSwingingOnRope _player false)
  (Variables|/Game/Game_Files/Characters/Main_Character/MainCharacterBP.MainCharacterBP_C|SetCan%20move? _player true)
  (Pawn|Components|CharacterMovement|SetMovementMode (Variables|/Script/Engine.Character|GetCharacterMovement _player) "MOVE_Walking" 0)
  (Animation|StopAnimMontage _player "/Game/Game_Files/Characters/Main_Character/Animations/RopeHang_Montage.RopeHang_Montage")
  (Class|PrimitiveComponent|SetLinearDamping (Variables|Default|GetJoint) 2.0)
  (Class|PrimitiveComponent|SetLinearDamping (Variables|Default|GetCable%20end) 2.0)
  (Collision|SetCollisionObjectType _capsule "ECC_WorldStatic")
  (Utilities|FlowControl|Delay 2.0)
  (Collision|SetCollisionObjectType _capsule "ECC_GameTraceChannel3"))

(event EventTick
  (params (DeltaSeconds :type Float%20%28single-precision%29))
  (bind _cable_end (Variables|Default|GetCable%20end))
  (bind _returnvalue (Transformation|GetWorldLocation _cable_end))
  (Variables|Default|SetPlayerPositionTransform (Math|Vector|MakeVector (.x _returnvalue) (.y _returnvalue) 0.0)))

(event EventBeginPlay
  (CallFunction|AddPhysicsContraint (Transformation|GetRelativeTransform (Variables|Default|GetCable%20start))))

(event EventOnInteracted
  (params (Player :type Main%20Character%20BP%20Object%20Reference) (Interacter :type Actor%20Object%20Reference) (IsUsingGamepad :type Boolean))
  (bind _playerpositiontransform (Variables|Default|GetPlayerPositionTransform))
  (Components|DestroyComponent (Variables|Default|GetPhysicsContraint2))
  (bind _output_get (Variables|Default|SetPlayer Player))
  (Rendering|SetVisibility (Variables|/Game/Game_Files/Characters/Main_Character/MainCharacterBP.MainCharacterBP_C|GetShield _output_get) false false)
  (Rendering|SetVisibility (Variables|/Game/Game_Files/Characters/Main_Character/MainCharacterBP.MainCharacterBP_C|GetWeapon _output_get) false false)
  (Variables|/Game/Game_Files/Characters/Main_Character/MainCharacterBP.MainCharacterBP_C|SetIsHidingWeapon (Variables|Default|GetPlayer) false)
  (Variables|/Game/Game_Files/Characters/Main_Character/MainCharacterBP.MainCharacterBP_C|SetRope (Variables|Default|GetPlayer) self)
  (Variables|Default|SetLastPlayerForwardVector (Transformation|GetActorForwardVector (Variables|Default|GetPlayer)))
  (Variables|Default|SetLastActorVelocity (Variables|/Game/Game_Files/Characters/Main_Character/MainCharacterBP.MainCharacterBP_C|GetSpeedOfCharacter _output_get))
  (Variables|/Game/Game_Files/Characters/Main_Character/MainCharacterBP.MainCharacterBP_C|SetBirdViewOn? (Variables|Default|GetPlayer) false)
  (Variables|/Game/Game_Files/Characters/Main_Character/MainCharacterBP.MainCharacterBP_C|SetCan%20move? (Variables|Default|GetPlayer) false)
  (Components|Movement|StopMovementImmediately (Variables|/Script/Engine.Character|GetCharacterMovement (Variables|Default|GetPlayer)))
  (Pawn|Components|CharacterMovement|SetMovementMode (Variables|/Script/Engine.Character|GetCharacterMovement (Variables|Default|GetPlayer)) "MOVE_Flying" 0)
  (Transformation|SetActorLocation (Variables|Default|GetPlayer) (Math|Vector|MakeVector (.x _playerpositiontransform) (.y _playerpositiontransform) (- (.z (Transformation|GetActorLocation (Variables|Default|GetPlayer))) 5e+01)) false false)
  (CallFunction|AddPhysicsContraint (Transformation|GetRelativeTransform (Variables|Default|GetCable%20start)))
  (Transformation|AttachComponentToComponent (Variables|Default|GetPlayer) (Variables|Default|GetJoint) "None" "KeepWorld" "KeepWorld" "KeepWorld" true)
  (Variables|/Game/Game_Files/Characters/Main_Character/MainCharacterBP.MainCharacterBP_C|SetIsSwingingOnRope (Variables|Default|GetPlayer) true)
  (bind _current_interact_widget (Variables|/Game/Game_Files/Characters/Main_Character/MainCharacterBP.MainCharacterBP_C|GetCurrent%20Interact%20Widget (Variables|Default|GetPlayer))
    (:then
      (Widget|RemovefromParent _current_interact_widget)
      (Variables|/Game/Game_Files/Characters/Main_Character/MainCharacterBP.MainCharacterBP_C|SetCurrent%20Interact%20Widget (Variables|Default|GetPlayer) 0)
      (Variables|/Game/Game_Files/Characters/Main_Character/MainCharacterBP.MainCharacterBP_C|SetWidgetParentObject (Variables|Default|GetPlayer) 0)
      (Animation|PlayAnimMontage (Variables|Default|GetPlayer) "/Game/Game_Files/Characters/Main_Character/Animations/RopeHang_Montage.RopeHang_Montage" 1.0 "Default")
      (Class|PrimitiveComponent|SetLinearDamping (Variables|Default|GetJoint) 0.06)
      (Class|PrimitiveComponent|SetLinearDamping (Variables|Default|GetCable%20end) 0.5)
      (CallFunction|AddSwingingForce (* (Variables|Default|GetLastPlayerForwardVector) (* (/ (Variables|Default|GetLastActorVelocity) 3e+02) 5e+01)) 1.0))
    (:else)))

(fn ConstructionScript
  (bind _rope_length (Variables|Default|GetRope%20Length))
  (bind _cable_end (Variables|Default|GetCable%20end))
  (bind _returnvalue (Transformation|GetWorldLocation _cable_end))
  (Transformation|SetRelativeLocation (Variables|Default|GetCable%20end) (Math|Vector|MakeVector 0.0 0.0 (Variables|Default|GetRope%20Length)) false false)
  (Variables|Default|SetPlayerPositionTransform (Math|Vector|MakeVector (.x _returnvalue) (.y _returnvalue) 0.0))
  (Components|Capsule|SetCapsuleHalfHeight (Variables|Default|GetCapsule) (/ _rope_length -4.0) true)
  (Transformation|SetRelativeLocation (Variables|Default|GetCapsule) (Math|Vector|MakeVector 0.0 0.0 (* (/ _rope_length -1e+02) 225.0)) false false))

(fn AddPhysicsContraint
  (params (TargetTransform :type Transform))
  (Variables|Default|GetPlayer
    (:then
      (bind _output_get (LocalVariables|SetJointOffset (- (- (.z (Transformation|GetActorLocation)) (.z (Transformation|GetActorLocation (Variables|Default|GetPlayer)))) 1e+02)))
      (bind _returnvalue (AddComponent|AddStaticMeshComponent false (Math|Transform|MakeTransform (Math|Vector|MakeVector (.x (.location TargetTransform)) (.y (.location TargetTransform)) (- (.z (.location TargetTransform)) _output_get)) "0, 0, 0" "0.100000,0.100000,0.100000")))
      (Variables|Default|SetJoint _returnvalue))
    (:else
      (LocalVariables|SetJointOffset 0.0)
      (bind _returnvalue_2 (AddComponent|AddStaticMeshComponent false (Math|Transform|MakeTransform (.location TargetTransform) "0, 0, 0" "0.100000,0.100000,0.100000")))
      (Variables|Default|SetJoint _returnvalue_2)))
  (Physics|SetSimulatePhysics (Variables|Default|GetJoint) true)
  (Physics|SetEnableGravity (Variables|Default|GetJoint) true)
  (Collision|SetCollisionResponsetoAllChannels (Variables|Default|GetJoint) "ECR_Ignore")
  (bind _returnvalue_3 (Game|AddComponentbyClass "/Script/Engine.PhysicsConstraintComponent" false TargetTransform))
  (bind _output_get_2 (Variables|Default|SetPhysicsContraint1 _returnvalue_3))
  (Class|PhysicsConstraintComponent|SetConstrainedComponents _output_get_2 (Variables|Default|GetCable%20start) "None" (Variables|Default|GetJoint) "None")
  (bind _returnvalue_4 (Game|AddComponentbyClass "/Script/Engine.PhysicsConstraintComponent" false (Math|Transform|MakeTransform (Math|Vector|MakeVector (.x (.location TargetTransform)) (.y (.location TargetTransform)) (- (.z (.location TargetTransform)) (LocalVariables|GetJointOffset))) "0, 0, 0" "1,1,1")))
  (bind _output_get_3 (Variables|Default|SetPhysicsContraint2 _returnvalue_4))
  (Class|PhysicsConstraintComponent|SetAngularTwistLimit _output_get_3 "ACM_Limited" 0.0)
  (Class|PhysicsConstraintComponent|SetAngularSwing1Limit _output_get_3 "ACM_Limited" 0.0)
  (Class|PhysicsConstraintComponent|SetAngularSwing2Limit _output_get_3 "ACM_Limited" 0.0)
  (Class|PhysicsConstraintComponent|SetConstrainedComponents _output_get_3 (Variables|Default|GetJoint) "None" (Variables|Default|GetCable%20end) "None")
  (Transformation|SetRelativeLocation (Variables|Default|GetCable1) (.location TargetTransform) false false)
  (Class|CableComponent|SetAttachEndtoComponent (Variables|Default|GetCable1) (Variables|Default|GetJoint) "None")
  (Transformation|SetRelativeLocation (Variables|Default|GetCable2) (Math|Vector|MakeVector (.x (.location TargetTransform)) (.y (.location TargetTransform)) (- (.z (.location TargetTransform)) (LocalVariables|GetJointOffset))) false false)
  (Class|CableComponent|SetAttachEndtoComponent (Variables|Default|GetCable2) (Variables|Default|GetCable%20end) "None")
  (Variables|/Script/CableComponent.CableComponent|SetEndLocation (Variables|Default|GetCable1) "0, 0, 0")
  (Variables|/Script/CableComponent.CableComponent|SetEndLocation (Variables|Default|GetCable2) "0, 0, 0")
  (Transformation|AttachComponentToComponent (Variables|Default|GetCable2) (Variables|Default|GetJoint) "None" "SnapToTarget" "KeepWorld" "KeepWorld" true))