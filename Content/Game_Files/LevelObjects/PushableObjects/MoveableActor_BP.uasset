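; Pushable level object that the player interacts with to start pushing and that can topple off edges.
; Interaction snaps the character to the nearest PushTransform, after space and walkable-floor checks, and hands off to its PushComponent.
; When IsFalling is set, Tick plays an edge-push montage, then launches the mesh with physics and an impulse, ignoring climb/push channels.
; Once velocity reaches zero, physics and Tick switch off and original climb/push collision returns.
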(event EventTick
  (params (DeltaSeconds :type Float%20%28single-precision%29))
  (bind _pushtransforms (Variables|Default|GetPushTransforms))
  (bind _closest_index (Variables|Default|GetClosest%20Index))
  (bind _mesh (Variables|Default|GetMesh))
  (bind _player (Variables|Default|GetPlayer))
  (bind _output (Utilities|Array|Get(acopy) _pushtransforms _closest_index))
  (Development|PrintString (Utilities|String|ToString(Float) (Math|Vector|VectorLength (Transformation|GetVelocity))))
  (Utilities|FlowControl|Sequence
    (:then_0
      (if (Variables|Default|GetIsFalling?)
        (Utilities|FlowControl|DoOnce false :!label _label
          (:Completed
            (Transformation|SetActorLocation _player (+ (* (Transformation|GetActorForwardVector _player) -2e+01) (Transformation|GetActorLocation _player)) false false)
            (Animation|PlayAnimMontage (Variables|Default|GetPlayer) "/Game/Game_Files/Characters/Main_Character/Animations/Push_from_edge_Montage.Push_from_edge_Montage" 1.0 "None")
            (Utilities|FlowControl|Delay 1.7)
            (Physics|SetSimulatePhysics (Variables|Default|GetMesh) true)
            (Variables|Default|SetCurrent%20Location%20of%20Closest%20Transform (Math|Transform|TransformLocation (Transformation|GetActorTransform) (.location _output)))
            (Variables|Default|SetCurrent%20Actor%20Location (Transformation|GetActorLocation))
            (Physics|AddImpulse (Variables|Default|GetMesh) (* (Math|Vector|GetForwardVector (Math|Transform|TransformRotation (Transformation|GetActorTransform) (.rotation _output))) (Variables|Default|GetPush%20Force%20Multiplier)) "None" false)
            (Collision|SetCollisionResponsetoChannel _mesh "ECC_GameTraceChannel1" "ECR_Ignore")
            (Collision|SetCollisionResponsetoChannel _mesh "ECC_GameTraceChannel2" "ECR_Ignore")
            (Utilities|FlowControl|Delay 1.0)
            (Variables|Default|SetCan%20Check%20for%20floor true)))
        (else
          (goto _label Reset))))
    (:then_1
      (if (Variables|Default|GetCan%20Check%20for%20floor)
        (CallFunction|CheckforFloorHit)))))

(event EventBeginPlay
  (Actor|Tick|SetActorTickEnabled false)
  (Utilities|GetMeshDimensions)
  (Variables|Default|SetIsFalling? false)
  (Physics|SetSimulatePhysics (Variables|Default|GetMesh) false)
  (CallFunction|CheckHeightfromPivottoFloor)
  (if (Utilities|Enum|Equal(Enum) (Utilities|String|EnumtoString (Collision|GetCollisionResponsetoChannel (Variables|Default|GetMesh) "ECC_GameTraceChannel1")) "Block")
    (Variables|Default|SetIs%20Climbable true)
    (else
      (Variables|Default|SetIs%20Climbable false)))
  (if (Utilities|Enum|Equal(Enum) (Utilities|String|EnumtoString (Collision|GetCollisionResponsetoChannel (Variables|Default|GetMesh) "ECC_GameTraceChannel2")) "Block")
    (Variables|Default|SetIs%20Pushable true)
    (else
      (Variables|Default|SetIs%20Pushable false))))

(event EventOnInteracted
  (params (Player :type Main%20Character%20BP%20Object%20Reference) (Interacter :type Actor%20Object%20Reference) (IsUsingGamepad :type Boolean))
  (Actor|Tick|SetActorTickEnabled true)
  (bind _output_get (Variables|Default|SetPlayer Player))
  (CallFunction|HandleInteraction _output_get))

(fn ConstructionScript
  (for _array_element (Variables|Default|GetPushTransforms)
    (AddComponent|AddArrowComponent false _array_element)))

(fn HandleInteraction
  (params (Character :type Character%20Object%20Reference))
  (bind _returnvalue (Transformation|GetActorTransform))
  (bind _output_get (LocalVariables|SetCharacterVar Character))
  (if (not (AI|Components|NavMovement|IsFalling (Variables|/Script/Engine.Character|GetCharacterMovement _output_get)))
    (Utilities|IsValid _output_get
      (:Is%20Valid
        (bind _output_get_2 (LocalVariables|SetPushComponent (Actor|GetComponentbyClass _output_get "/Game/Game_Files/Characters/Main_Character/PushComponent.PushComponent_C")))
        (Utilities|IsValid _output_get_2
          (:Is%20Valid
            (bind _closestindex (CallFunction|FindClosestPushTransformIndex (Math|Conversions|ToVector2D(Vector) (Transformation|GetActorLocation (LocalVariables|GetCharacterVar))) (Variables|/Game/Game_Files/Characters/Main_Character/PushComponent.PushComponent_C|GetPushRange (LocalVariables|GetPushComponent))))
            (Variables|Default|SetClosest%20Index _closestindex)
            (if (>= _closestindex 0)
              (bind _output_get_3 (LocalVariables|SetCharacterNewTransform (Math|Transform|MakeTransform (+ (.location (Math|Transform|ComposeTransforms (Utilities|Array|Get(acopy) (Variables|Default|GetPushTransforms) _closestindex) (Transformation|GetActorTransform))) (Math|Vector|MakeVector 0.0 0.0 (Components|Capsule|GetScaledCapsuleHalfHeight (Variables|/Script/Engine.Character|GetCapsuleComponent Character)))) (.rotation (Math|Transform|ComposeTransforms (Utilities|Array|Get(acopy) (Variables|Default|GetPushTransforms) _closestindex) (Transformation|GetActorTransform))) (.scale (Transformation|GetActorTransform (LocalVariables|GetCharacterVar))))))
              (Rendering|Debug|DrawDebugSphere (.location _output_get_3) 2e+01 12 "(R=1.000000,G=0.000000,B=0.056108,A=1.000000)" 2.0 1.0)
              (bind _outhit (Collision|CapsuleTraceByChannel (+ (.location (LocalVariables|GetCharacterNewTransform)) "0, 0,70.000000") (- (.location (LocalVariables|GetCharacterNewTransform)) "0, 0,100.000000") (Components|Capsule|GetScaledCapsuleRadius (Variables|/Script/Engine.Character|GetCapsuleComponent (LocalVariables|GetCharacterVar))) (Components|Capsule|GetScaledCapsuleHalfHeight (Variables|/Script/Engine.Character|GetCapsuleComponent (LocalVariables|GetCharacterVar))) "TraceTypeQuery1" false 0 "None" true "(R=1.000000,G=0.000000,B=0.000000,A=1.000000)" "(R=0.000000,G=1.000000,B=0.000000,A=1.000000)" 2.0))
              (if (not (.bInitialOverlap (Collision|BreakHitResult _outhit)))
                (if (< (Class|CharacterMovementComponent|GetWalkableFloorZ (Variables|/Script/Engine.Character|GetCharacterMovement (LocalVariables|GetCharacterVar))) (.Z (Math|Vector|BreakVector (.ImpactNormal (Collision|BreakHitResult _outhit)))))
                  (Transformation|SetActorTransform Character (Math|Transform|MakeTransform (.location (LocalVariables|GetCharacterNewTransform)) (.rotation (LocalVariables|GetCharacterNewTransform)) (.scale (LocalVariables|GetCharacterNewTransform))))
                  (Variables|/Game/Game_Files/Characters/Main_Character/UserInterface/InteractionWidget.InteractionWidget_C|SetText (Variables|/Game/Game_Files/Characters/Main_Character/MainCharacterBP.MainCharacterBP_C|GetCurrent%20Interact%20Widget (Variables|Default|GetPlayer)) (Utilities|Text|MakeLiteralText "Stop pushing"))
                  (Default|BeginPush (LocalVariables|GetPushComponent) self (Math|Transform|MakeTransform (Math|Transform|TransformLocation _returnvalue (.location (Utilities|Array|Get(acopy) (Variables|Default|GetPushTransforms) (Variables|Default|GetClosest%20Index)))) (Math|Transform|TransformRotation _returnvalue (.rotation (Utilities|Array|Get(acopy) (Variables|Default|GetPushTransforms) (Variables|Default|GetClosest%20Index)))) (.scale (Utilities|Array|Get(acopy) (Variables|Default|GetPushTransforms) (Variables|Default|GetClosest%20Index)))))
                  (else
                    (Utilities|PushFailedInfo "Surface is not walkable")))
                (else
                  (Utilities|PushFailedInfo "No enought space")))
              (else
                (Utilities|PushFailedInfo "No PushTransform Found"))))
          (:Is%20Not%20Valid
            (Utilities|PushFailedInfo "Character does not have PushComponent"))))
      (:Is%20Not%20Valid
        (Utilities|PushFailedInfo "Character is not valid")))))

(fn FindClosestPushTransformIndex
  (params (CharacterLocation :type Vector%202D%20Structure) (PushRange :type Float%20%28single-precision%29))
  (for (_array_element _array_index) (Variables|Default|GetPushTransforms)
    (LocalVariables|SetCurrentTransformIndex _array_index)
    (LocalVariables|SetTheCurrentDistance (Class|KismetMathLibrary|DistanceSquared2D (Math|Conversions|ToVector2D(Vector) (Math|Transform|TransformLocation (Transformation|GetActorTransform) (.location _array_element))) CharacterLocation))
    (if (<= (LocalVariables|GetCurrentTransformIndex) 0)
      (LocalVariables|SetClosestTransformIIndex (LocalVariables|GetCurrentTransformIndex) :!label _label)
      (LocalVariables|SetTheClosestDistance (LocalVariables|GetTheCurrentDistance))
      (elif (< (LocalVariables|GetTheCurrentDistance) (LocalVariables|GetTheClosestDistance))
        (goto _label))))
  (return (LocalVariables|GetClosestTransformIIndex)))

(fn CheckHeightfromPivottoFloor
  (bind _returnvalue (Transformation|GetActorLocation))
  (bind (_x _y _z) (Math|Vector|BreakVector _returnvalue))
  (bind _outhit (Collision|LineTraceByChannel _returnvalue (Math|Vector|MakeVector _x _y (- _z 2e+02)) "TraceTypeQuery1" false 0 "ForOneFrame"))
  (Variables|Default|SetPivotHeightFromFloor (- (.z (Transformation|GetActorLocation)) (.Z (Math|Vector|BreakVector (.location _outhit))))))

(fn CheckforFloorHit
  (bind _returnvalue (Transformation|GetActorLocation))
  (bind _mesh (Variables|Default|GetMesh))
  (bind _mesh_2 (Variables|Default|GetMesh))
  (if (not (> (Math|Vector|VectorLength (Transformation|GetVelocity)) 0.0))
    (Physics|SetSimulatePhysics (Variables|Default|GetMesh) false)
    (if (Variables|Default|GetIs%20Climbable)
      (Collision|SetCollisionResponsetoChannel _mesh_2 "ECC_GameTraceChannel1" "ECR_Block")
      (else
        (Collision|SetCollisionResponsetoChannel _mesh "ECC_GameTraceChannel1" "ECR_Ignore")))
    (if (Variables|Default|GetIs%20Pushable)
      (Collision|SetCollisionResponsetoChannel _mesh_2 "ECC_GameTraceChannel2" "ECR_Block")
      (else
        (Collision|SetCollisionResponsetoChannel _mesh "ECC_GameTraceChannel2" "ECR_Ignore")))
    (Variables|Default|SetIsFalling? false)
    (Variables|Default|SetCan%20Check%20for%20floor false)
    (Transformation|SetActorLocation (Math|Vector|MakeVector (.x _returnvalue) (.y _returnvalue) (+ (.z _returnvalue) 2.0)) false false)
    (Actor|Tick|SetActorTickEnabled false)))