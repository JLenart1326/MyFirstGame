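; WoodenBasket_BP is an openable wooden basket container that animates its child mesh when opened or closed through interaction.
; The OpenOrClose timeline drives the mesh's relative yaw and X/Y position while keeping its height, playing forward to open and in reverse to close.
; Overridden child reaction functions trigger Open or Close, then call the parent interaction logic.
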(event Custom|Open
  (bind _staticmeshchild (Variables|Default|GetStaticMeshChild))
  (bind (_direction _yaw _y _x) (Timeline|Open%20or%20Close Play)
    (:Update
      (Transformation|SetRelativeRotation _staticmeshchild (Math|Rotator|MakeRotator 0.0 0.0 _yaw) false false)
      (Transformation|SetRelativeLocation _staticmeshchild (Math|Vector|MakeVector _x _y (.z (Variables|/Script/Engine.SceneComponent|GetRelativeLocation _staticmeshchild))) false false))))

(event Custom|Close
  (bind _staticmeshchild (Variables|Default|GetStaticMeshChild))
  (bind (_direction _yaw _y _x) (Timeline|Open%20or%20Close Reverse)
    (:Update
      (Transformation|SetRelativeRotation _staticmeshchild (Math|Rotator|MakeRotator 0.0 0.0 _yaw) false false)
      (Transformation|SetRelativeLocation _staticmeshchild (Math|Vector|MakeVector _x _y (.z (Variables|/Script/Engine.SceneComponent|GetRelativeLocation _staticmeshchild))) false false))))

(fn ConstructionScript
  (|CallParentFunction))

(fn InteractionChildReactionOpen
  (CallFunction|Open)
  (|CallParentFunction))

(fn InteractionChildReactionClose
  (CallFunction|Close)
  (|CallParentFunction))