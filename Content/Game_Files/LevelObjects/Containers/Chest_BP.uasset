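; Interactable chest that swings its lid open and closed and makes AI-audible noise attributed to the player.
; It overrides the parent's open and close interaction reactions, then calls the parent versions.
; The OpenOrClose timeline drives the child mesh's roll, playing forward to open and reversing to close.
; Noise events fire as opening starts and when closing finishes, each with a debug print.
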(event Custom|Open
  (Variables|Default|SetIsClosing false)
  (bind _row (Timeline|Open%20or%20Close Play)
    (:Update
      (Transformation|SetRelativeRotation (Variables|Default|GetStaticMeshChild) (Math|Rotator|MakeRotator _row 0.0 0.0) false false))
    (:Finished
      (if (Variables|Default|GetIsClosing)
        (Class|AISenseHearing|ReportNoiseEvent (Transformation|GetActorLocation) 1.0 (Variables|Default|GetPlayer) 0.0 "Noise")
        (Development|PrintString "Noise")))))

(event Custom|Close
  (Variables|Default|SetIsClosing true)
  (bind _row (Timeline|Open%20or%20Close Reverse)
    (:Update
      (Transformation|SetRelativeRotation (Variables|Default|GetStaticMeshChild) (Math|Rotator|MakeRotator _row 0.0 0.0) false false))
    (:Finished
      (if (Variables|Default|GetIsClosing)
        (Class|AISenseHearing|ReportNoiseEvent (Transformation|GetActorLocation) 1.0 (Variables|Default|GetPlayer) 0.0 "Noise")
        (Development|PrintString "Noise")))))

(fn ConstructionScript
  (|CallParentFunction))

(fn InteractionChildReactionOpen
  (Class|AISenseHearing|ReportNoiseEvent (Transformation|GetActorLocation) 1.0 (Variables|Default|GetPlayer) 0.0 "Noise")
  (Development|PrintString "Noise")
  (CallFunction|Open)
  (|CallParentFunction))

(fn InteractionChildReactionClose
  (CallFunction|Close)
  (|CallParentFunction))