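; Base Blueprint for interactable level containers that hold items in an inventory component.
; BeginPlay copies the Items array into the component's Inventory, index by index.
; Interaction fires an open-reaction hook, waits briefly, then toggles the inventory if the interacter is MainCharacterBP.
; Open and close reaction functions are empty stubs for child containers, and the close one is not called here.
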(event EventOnInteracted
  (params (Player :type Main%20Character%20BP%20Object%20Reference) (Interacter :type Actor%20Object%20Reference))
  (CallFunction|InteractionChildReactionOpen)
  (Utilities|FlowControl|Delay 0.5)
  (Utilities|Casting|CastToMainCharacterBP Interacter)
  (Default|ToogleInventory (Variables|Default|GetInventoryComponent)))

(event EventBeginPlay
  (for (_array_element _array_index) (Variables|Default|GetItems)
    (Utilities|Array|SetArrayElem (Variables|/Game/Game_Files/InventorySystem/InventoryComponent.InventoryComponent_C|GetInventory (Variables|Default|GetInventoryComponent)) _array_index _array_element)))

(fn ConstructionScript)

(fn InteractionChildReactionOpen
  (return))

(fn InteractionChildReactionClose)