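; TriggerBoxBP is a trigger volume that changes the main character's camera direction.
; On begin overlap, it casts the other actor to MainCharacterBP, stores the reference, and sets its CameraChange flag with Direction "FrontSide".
; On end overlap, it sets the flag again with Direction "LeftSide" on the stored reference, without checking which actor left.
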(event OnComponentBeginOverlap(Box)
  (params (OverlappedComponent :type Primitive%20Component%20Object%20Reference) (OtherActor :type Actor%20Object%20Reference) (OtherComp :type Primitive%20Component%20Object%20Reference) (OtherBodyIndex :type Integer) (bFromSweep :type Boolean) (SweepResult :type Hit%20Result%20Structure%20%28by%20ref%29))
  ;[1 1 1] Player Camera Change on Overlap
  (bind _asmain_character_bp (Utilities|Casting|CastToMainCharacterBP OtherActor))
  (Variables|Default|SetCharacterBPReference _asmain_character_bp)
  (Variables|/Game/Game_Files/Characters/MainCharacterBP.MainCharacterBP_C|SetCameraChange (Variables|Default|GetCharacterBPReference) true)
  (Variables|/Game/Game_Files/Characters/MainCharacterBP.MainCharacterBP_C|SetDirection (Variables|Default|GetCharacterBPReference) "FrontSide"))

(event OnComponentEndOverlap(Box)
  (params (OverlappedComponent :type Primitive%20Component%20Object%20Reference) (OtherActor :type Actor%20Object%20Reference) (OtherComp :type Primitive%20Component%20Object%20Reference) (OtherBodyIndex :type Integer))
  ;[1 1 1] Player Camera Change on Overlap
  (Variables|/Game/Game_Files/Characters/MainCharacterBP.MainCharacterBP_C|SetCameraChange (Variables|Default|GetCharacterBPReference) true)
  (Variables|/Game/Game_Files/Characters/MainCharacterBP.MainCharacterBP_C|SetDirection (Variables|Default|GetCharacterBPReference) "LeftSide"))

(fn ConstructionScript)