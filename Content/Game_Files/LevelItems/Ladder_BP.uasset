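; Climbable ladder actor that tells MainCharacterBP when it is nearby and moves a climbing character off at the end.
; Box overlap sets the character's near-ladder flag and actor reference; leaving clears them and the climbing flag and restores walking.
; EndClimbingBox moves a climbing character to the closest PositionTransforms point plus a fixed world X and Z offset.
; The construction script adds an arrow component at each of those points.
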(event OnComponentBeginOverlap(Box)
  (params (OverlappedComponent :type Primitive%20Component%20Object%20Reference) (OtherActor :type Actor%20Object%20Reference) (OtherComp :type Primitive%20Component%20Object%20Reference) (OtherBodyIndex :type Integer) (bFromSweep :type Boolean) (SweepResult :type Hit%20Result%20Structure%20%28by%20ref%29))
  (bind _asmain_character_bp (Utilities|Casting|CastToMainCharacterBP OtherActor))
  (Variables|/Game/Game_Files/Characters/Main_Character/MainCharacterBP.MainCharacterBP_C|SetNearTheLadder? _asmain_character_bp true)
  (Variables|/Game/Game_Files/Characters/Main_Character/MainCharacterBP.MainCharacterBP_C|SetOverlapedActor _asmain_character_bp self))

(event OnComponentEndOverlap(Box)
  (params (OverlappedComponent :type Primitive%20Component%20Object%20Reference) (OtherActor :type Actor%20Object%20Reference) (OtherComp :type Primitive%20Component%20Object%20Reference) (OtherBodyIndex :type Integer))
  (bind _asmain_character_bp (Utilities|Casting|CastToMainCharacterBP OtherActor))
  (Variables|/Game/Game_Files/Characters/Main_Character/MainCharacterBP.MainCharacterBP_C|SetNearTheLadder? _asmain_character_bp false)
  (Variables|/Game/Game_Files/Characters/Main_Character/MainCharacterBP.MainCharacterBP_C|SetOnLadder? _asmain_character_bp false)
  (Pawn|Components|CharacterMovement|SetMovementMode (Variables|/Script/Engine.Character|GetCharacterMovement _asmain_character_bp) "MOVE_Walking" 0)
  (Variables|/Game/Game_Files/Characters/Main_Character/MainCharacterBP.MainCharacterBP_C|SetOverlapedActor _asmain_character_bp 0))

(event OnComponentBeginOverlap(EndClimbingBox)
  (params (OverlappedComponent :type Primitive%20Component%20Object%20Reference) (OtherActor :type Actor%20Object%20Reference) (OtherComp :type Primitive%20Component%20Object%20Reference) (OtherBodyIndex :type Integer) (bFromSweep :type Boolean) (SweepResult :type Hit%20Result%20Structure%20%28by%20ref%29))
  (bind _asmain_character_bp (Utilities|Casting|CastToMainCharacterBP OtherActor))
  (if (Variables|/Game/Game_Files/Characters/Main_Character/MainCharacterBP.MainCharacterBP_C|GetOnLadder? _asmain_character_bp)
    (CallFunction|SetCharacterinCorrectPosition _asmain_character_bp)
    (else
      (Development|PrintString "Nie wspinasz sie"))))

(event OnComponentEndOverlap(EndClimbingBox)
  (params (OverlappedComponent :type Primitive%20Component%20Object%20Reference) (OtherActor :type Actor%20Object%20Reference) (OtherComp :type Primitive%20Component%20Object%20Reference) (OtherBodyIndex :type Integer))
  (Utilities|Casting|CastToMainCharacterBP OtherActor))

(fn ConstructionScript
  (for _array_element (Variables|Default|GetPositionTransforms)
    (AddComponent|AddArrowComponent false _array_element)))

(fn FindClosestClimbIndex
  (params (CharacterLocation :type Vector))
  (for (_array_element _array_index) (Variables|Default|GetPositionTransforms)
    (LocalVariables|SetCurrentTransformIndex _array_index)
    (LocalVariables|SetTheCurrentDistance (Class|KismetMathLibrary|VectorDistanceSquared (Math|Transform|TransformLocation (Transformation|GetActorTransform) (.location _array_element)) CharacterLocation))
    (if (<= (LocalVariables|GetCurrentTransformIndex) 0)
      (LocalVariables|SetClosestTransformIIndex (LocalVariables|GetCurrentTransformIndex) :!label _label)
      (LocalVariables|SetTheClosestDistance (LocalVariables|GetTheCurrentDistance))
      (elif (< (LocalVariables|GetTheCurrentDistance) (LocalVariables|GetTheClosestDistance))
        (goto _label))))
  (return (LocalVariables|GetClosestTransformIIndex)))

(fn SetCharacterinCorrectPosition
  (params (Character :type Main%20Character%20BP%20Object%20Reference))
  (LocalVariables|SetClimbingCharacter Character)
  (bind _closestindex (CallFunction|FindClosestClimbIndex (Transformation|GetActorLocation Character)))
  (Transformation|SetActorLocation (LocalVariables|GetClimbingCharacter) (Math|Vector|MakeVector (+ (.x (Math|Transform|TransformLocation (Transformation|GetActorTransform) (.location (Utilities|Array|Get(acopy) (Variables|Default|GetPositionTransforms) _closestindex)))) 1e+02) (.y (Math|Transform|TransformLocation (Transformation|GetActorTransform) (.location (Utilities|Array|Get(acopy) (Variables|Default|GetPositionTransforms) _closestindex)))) (+ (.z (Math|Transform|TransformLocation (Transformation|GetActorTransform) (.location (Utilities|Array|Get(acopy) (Variables|Default|GetPositionTransforms) _closestindex)))) 2e+02)) false false))