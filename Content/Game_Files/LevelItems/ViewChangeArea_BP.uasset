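; ViewChangeArea_BP is a level trigger volume that switches the main character's camera direction while the player is inside it.
; On overlap it saves the old direction, applies NewDirection, and blocks movement for 1.5 seconds.
; It then widens the box in X and Y, so the exit boundary sits beyond the entry one.
; End overlap, without an actor check, restores the direction, pauses movement again and resets the box scale.
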(event OnComponentBeginOverlap(Box)
  (params (OverlappedComponent :type Primitive%20Component%20Object%20Reference) (OtherActor :type Actor%20Object%20Reference) (OtherComp :type Primitive%20Component%20Object%20Reference) (OtherBodyIndex :type Integer) (bFromSweep :type Boolean) (SweepResult :type Hit%20Result%20Structure%20%28by%20ref%29))
  (bind _box (Variables|Default|GetBox))
  (bind _returnvalue (Transformation|GetRelativeTransform _box))
  (bind (_x _y _z) (Math|Vector|BreakVector (.scale _returnvalue)))
  ;[1 1 1] Player Camera Change on Overlap
  (bind _asmain_character_bp (Utilities|Casting|CastToMainCharacterBP OtherActor))
  (Variables|Default|SetCharacterBPReference _asmain_character_bp)
  (Variables|Default|SetCharacter%20Movement (Variables|/Script/Engine.Character|GetCharacterMovement _asmain_character_bp))
  (Variables|/Game/Game_Files/Characters/Main_Character/MainCharacterBP.MainCharacterBP_C|SetCameraChange (Variables|Default|GetCharacterBPReference) true)
  (Variables|Default|SetOldDirection (Variables|/Game/Game_Files/Characters/Main_Character/MainCharacterBP.MainCharacterBP_C|GetCameraDirection (Variables|Default|GetCharacterBPReference)))
  (Variables|/Game/Game_Files/Characters/Main_Character/MainCharacterBP.MainCharacterBP_C|SetCameraDirection (Variables|Default|GetCharacterBPReference) (Variables|Default|GetNewDirection))
  (Variables|/Game/Game_Files/Characters/Main_Character/MainCharacterBP.MainCharacterBP_C|SetCan%20move? (Variables|Default|GetCharacterBPReference) false)
  (Utilities|FlowControl|Delay 1.5)
  (Variables|Default|SetPrimaryScale (.scale _returnvalue))
  (Transformation|SetRelativeTransform _box (Math|Transform|MakeTransform (.location _returnvalue) (.rotation _returnvalue) (Math|Vector|MakeVector (* _x 1.5) (* _y 1.5) _z)) false false)
  (Variables|/Game/Game_Files/Characters/Main_Character/MainCharacterBP.MainCharacterBP_C|SetCan%20move? (Variables|Default|GetCharacterBPReference) true))

(event OnComponentEndOverlap(Box)
  (params (OverlappedComponent :type Primitive%20Component%20Object%20Reference) (OtherActor :type Actor%20Object%20Reference) (OtherComp :type Primitive%20Component%20Object%20Reference) (OtherBodyIndex :type Integer))
  (bind _box (Variables|Default|GetBox))
  (bind _returnvalue (Transformation|GetRelativeTransform _box))
  ;[1 1 1] Player Camera Change on Overlap
  (Variables|/Game/Game_Files/Characters/Main_Character/MainCharacterBP.MainCharacterBP_C|SetCameraChange (Variables|Default|GetCharacterBPReference) true)
  (Variables|/Game/Game_Files/Characters/Main_Character/MainCharacterBP.MainCharacterBP_C|SetCameraDirection (Variables|Default|GetCharacterBPReference) (Variables|Default|GetOldDirection))
  (Variables|/Game/Game_Files/Characters/Main_Character/MainCharacterBP.MainCharacterBP_C|SetCan%20move? (Variables|Default|GetCharacterBPReference) false)
  (Utilities|FlowControl|Delay 1.5)
  (Transformation|SetRelativeTransform _box (Math|Transform|MakeTransform (.location _returnvalue) (.rotation _returnvalue) (Variables|Default|GetPrimaryScale)) false false)
  (Variables|/Game/Game_Files/Characters/Main_Character/MainCharacterBP.MainCharacterBP_C|SetCan%20move? (Variables|Default|GetCharacterBPReference) true))

(fn ConstructionScript)