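; Inventory UI 3D capture actor that mirrors the player character's appearance and equipped gear.
; On BeginPlay, UpdateMesh copies the skeletal mesh from MainCharacterBP plus its helmet, weapon, shield and body static meshes.
; Each gear piece then snaps to its head, hand or spine socket on the duplicate skeleton.
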(event Custom|UpdateMesh
  (bind _asmain_character_bp (Utilities|Casting|CastToMainCharacterBP (Game|GetPlayerCharacter 0)))
  (Variables|Default|SetPlayer _asmain_character_bp)
  (Class|SkinnedMeshComponent|SetSkeletalMesh (Variables|Default|GetSkeletalMesh) (Variables|/Script/Engine.SkinnedMeshComponent|GetSkeletalMesh (Variables|/Script/Engine.Character|GetMesh _asmain_character_bp)) true)
  (Components|StaticMesh|SetStaticMesh (Variables|Default|GetHelmet) (Variables|/Script/Engine.StaticMeshComponent|GetStaticMesh (Variables|/Game/Game_Files/Characters/Main_Character/MainCharacterBP.MainCharacterBP_C|GetHelmet (Variables|Default|GetPlayer))))
  (Components|StaticMesh|SetStaticMesh (Variables|Default|GetWeapon) (Variables|/Script/Engine.StaticMeshComponent|GetStaticMesh (Variables|/Game/Game_Files/Characters/Main_Character/MainCharacterBP.MainCharacterBP_C|GetWeapon (Variables|Default|GetPlayer))))
  (Components|StaticMesh|SetStaticMesh (Variables|Default|GetShield) (Variables|/Script/Engine.StaticMeshComponent|GetStaticMesh (Variables|/Game/Game_Files/Characters/Main_Character/MainCharacterBP.MainCharacterBP_C|GetShield (Variables|Default|GetPlayer))))
  (Components|StaticMesh|SetStaticMesh (Variables|Default|GetBody) (Variables|/Script/Engine.StaticMeshComponent|GetStaticMesh (Variables|/Game/Game_Files/Characters/Main_Character/MainCharacterBP.MainCharacterBP_C|GetBody (Variables|Default|GetPlayer))))
  (Transformation|AttachComponentToComponent (Variables|Default|GetHelmet) (Variables|Default|GetSkeletalMesh) "headSocket" "SnapToTarget" "SnapToTarget" "SnapToTarget" true)
  (Transformation|AttachComponentToComponent (Variables|Default|GetWeapon) (Variables|Default|GetSkeletalMesh) "hand_rSocket" "SnapToTarget" "SnapToTarget" "SnapToTarget" true)
  (Transformation|AttachComponentToComponent (Variables|Default|GetShield) (Variables|Default|GetSkeletalMesh) "hand_lSocket" "SnapToTarget" "SnapToTarget" "SnapToTarget" true)
  (Transformation|AttachComponentToComponent (Variables|Default|GetBody) (Variables|Default|GetSkeletalMesh) "spine_03Socket" "SnapToTarget" "SnapToTarget" "SnapToTarget" true))

(event EventBeginPlay
  (CallFunction|UpdateMesh))

(fn ConstructionScript)